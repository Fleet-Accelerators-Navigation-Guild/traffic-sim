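; Race manager that runs the start countdown and builds the checkpoint loop for a track.
; On BeginPlay it shows a countdown widget, freezes the listed cars, then after a fixed delay frees them and activates checkpoints.
; Checkpoints are spawned at regular gaps along the Road spline, facing its direction and linked into a closed ring through NextCheckpoint.
; Only the first checkpoint is switched on.
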(event EventBeginPlay
  (bind _returnvalue (UserInterface|CreateWidget "/Game/Blueprints/UI/WDG_CountDown.WDG_CountDown_C"))
  (Default|StartCountDown _returnvalue 3 "GO!")
  (UserInterface|Viewport|AddtoViewport _returnvalue 0)
  (CallFunction|ToggleCarsMovement false)
  (Utilities|FlowControl|Delay 4.0)
  (CallFunction|ToggleCarsMovement true)
  (|ActivateCheckpoints))

(event Collision|EventActorBeginOverlap
  (params (OtherActor :type Actor%20Object%20Reference)))

(event EventTick
  (params (DeltaSeconds :type Float%20%28single-precision%29)))

(fn ConstructionScript)

(fn ToggleCarsMovement
  (params (MovementEnabled :type Boolean))
  (for _array_element (Variables|Default|GetCars)
    (Variables|/Game/VehicleTemplate/Blueprints/SportsCar/SportsCar_Pawn.SportsCar_Pawn_C|SetMovementEnabled _array_element MovementEnabled)))

(fn PlaceCheckpoints
  (bind _checkpoints (Variables|Default|GetCheckpoints))
  (bind _checkpoints_2 (Variables|Default|GetCheckpoints))
  (CallFunction|ClearCheckpoints)
  (bind _road (Variables|Default|GetRoad)
    (:then
      (if (> (Spline|GetSplineLength (Variables|/Game/Blueprints/BP_Road.BP_Road_C|GetSpline _road)) (LocalVariables|GetCheckpointDistance)) :!label _label
        (bind _returnvalue (Game|SpawnActorfromClass "/Game/Blueprints/Checkpoint/BP_Checkpoint.BP_Checkpoint_C" (Math|Transform|MakeTransform (Spline|GetLocationatDistanceAlongSpline (Variables|/Game/Blueprints/BP_Road.BP_Road_C|GetSpline _road) (LocalVariables|GetCheckpointDistance) "World") (Math|Conversions|RotationFromXVector (Spline|GetDirectionatDistanceAlongSpline (Variables|/Game/Blueprints/BP_Road.BP_Road_C|GetSpline _road) (LocalVariables|GetCheckpointDistance) "World")) "1.000000,1.000000,1.000000") "AlwaysSpawn" "MultiplyWithRoot" 0 0))
        (bind _returnvalue_2 (Utilities|Array|Add _checkpoints _returnvalue))
        (if (> _returnvalue_2 0)
          (Variables|/Game/Blueprints/Checkpoint/BP_Checkpoint.BP_Checkpoint_C|SetNextCheckpoint (Utilities|Array|Get(acopy) _checkpoints (- _returnvalue_2 1)) (Utilities|Array|Get(acopy) _checkpoints _returnvalue_2)))
        (LocalVariables|SetCheckpointDistance (+ (LocalVariables|GetCheckpointDistance) (Variables|Default|GetCheckpointGap)))
        (goto _label)
        (else
          (Variables|/Game/Blueprints/Checkpoint/BP_Checkpoint.BP_Checkpoint_C|SetNextCheckpoint (Utilities|Array|Get(acopy) _checkpoints_2 (Utilities|Array|LastIndex _checkpoints_2)) (Utilities|Array|Get(acopy) _checkpoints_2))
          (return))))
    (:else)))

(fn ClearCheckpoints
  (bind _checkpoints (Variables|Default|GetCheckpoints))
  (for _array_element _checkpoints
    (Actor|SetLifeSpan _array_element 0.1))
  (Utilities|Array|Clear _checkpoints))