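; BP_Road is a spline road actor that can record a reference car's speed profile and serve it as ideal speed by track distance.
; With RecordSpeed on, a looping timer maps the car's closest spline distance to its speed and draws debug markers, stopping near the spline's end.
; Closest distance comes from fixed-step spline sampling.
; GetIdealSpeed returns the nearest recorded speed, scanning keys with an early exit that assumes distance order.
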(event EventBeginPlay
  (if (Variables|Default|GetRecordSpeed)
    (Utilities|Time|SetTimerbyFunctionName 0 "Record" 0.5 true)))

(event Collision|EventActorBeginOverlap
  (params (OtherActor :type Actor%20Object%20Reference)))

(event EventTick
  (params (DeltaSeconds :type Float%20%28single-precision%29)))

(fn ConstructionScript)

(fn Record
  (bind _referencecar (Variables|Default|GetReferenceCar))
  (bind _closessplinelength (CallFunction|FindClosestPointonRoad (Transformation|GetActorLocation _referencecar)))
  (Utilities|Map|Add (Variables|Default|GetSpeedAtDistance) _closessplinelength (Math|Vector|VectorLength (Transformation|GetVelocity _referencecar)))
  (Rendering|Debug|DrawDebugLine :LineStart (Spline|GetLocationatDistanceAlongSpline (Variables|Default|GetSpline) _closessplinelength "World") :LineEnd (+ (Spline|GetLocationatDistanceAlongSpline (Variables|Default|GetSpline) _closessplinelength "World") "0.000000,0.000000,500.000000") :Duration 5.0 :Thickness 1e+01)
  (if (Math|Float|NearlyEqual(Float) _closessplinelength (Spline|GetSplineLength (Variables|Default|GetSpline)) 5e+02)
    (Utilities|Time|ClearTimerbyFunctionName 0 "Record")))

(fn FindClosestPointonRoad
  (params (Location :type Vector))
  (bind _spline (Variables|Default|GetSpline))
  (if (< (LocalVariables|GetDistance) (Spline|GetSplineLength _spline)) :!label _label
    (if (< (Math|Vector|Distance(Vector) Location (Spline|GetLocationatDistanceAlongSpline _spline (LocalVariables|GetDistance) "World")) (LocalVariables|GetClosestDifference))
      (LocalVariables|SetClosestDistance (LocalVariables|GetDistance))
      (LocalVariables|SetClosestDifference (Math|Vector|Distance(Vector) Location (Spline|GetLocationatDistanceAlongSpline _spline (LocalVariables|GetDistance) "World"))))
    (LocalVariables|SetDistance (+ (LocalVariables|GetDistance) 2.5e+02))
    (goto _label)
    (else
      (return (LocalVariables|GetClosestDistance)))))

(fn GetIdealSpeed
  (params (SplineDistance :type Float%20%28double-precision%29))
  (bind _keys (Utilities|Map|Keys (Variables|Default|GetSpeedAtDistance)))
  (LocalVariables|SetMinDelta (Math|Float|Absolute(Float) (- (Utilities|Array|Get(acopy) _keys) SplineDistance)))
  (LocalVariables|SetClosestSplineDistance (Utilities|Array|Get(acopy) _keys))
  (bind _array_element (Utilities|Array|ForEachLoopwithBreak _keys :!label _label)
    (:LoopBody
      (if (> (Math|Float|Absolute(Float) (- _array_element SplineDistance)) (LocalVariables|GetMinDelta))
        (goto _label Break)
        (else
          (LocalVariables|SetMinDelta (Math|Float|Absolute(Float) (- _array_element SplineDistance)))
          (LocalVariables|SetClosestSplineDistance _array_element))))
    (:Completed
      (return (.Value (Utilities|Map|Find (Variables|Default|GetSpeedAtDistance) (LocalVariables|GetClosestSplineDistance)))))))