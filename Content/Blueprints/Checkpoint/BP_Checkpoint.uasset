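; BP_Checkpoint is a checkpoint actor that forms a chain, handing activation to the next one as the player reaches it.
; ToggleCheckpoint stores the Active flag and sets both visibility and the collider's query collision from it, starting with the initial value on BeginPlay.
; When an overlapping actor passes the IsPlayerMessage check, the checkpoint deactivates itself and activates NextCheckpoint if that reference is valid.
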(event OnComponentBeginOverlap(CheckpointCollider)
  (params (OverlappedComponent :type Primitive%20Component%20Object%20Reference) (OtherActor :type Actor%20Object%20Reference) (OtherComp :type Primitive%20Component%20Object%20Reference) (OtherBodyIndex :type Integer) (bFromSweep :type Boolean) (SweepResult :type Hit%20Result%20Structure%20%28by%20ref%29))
  (bind _yes_no (Class|BPICar|IsPlayer(Message) OtherActor))
  (if _yes_no
    (CallFunction|ToggleCheckpoint false)
    (bind _nextcheckpoint (Variables|Default|GetNextCheckpoint)
      (:then
        (CallFunction|ToggleCheckpoint _nextcheckpoint true))
      (:else))))

(event Custom|ToggleCheckpoint
  (params (Active :type Boolean))
  (bind _checkpointcollider (Variables|Default|GetCheckpointCollider))
  (bind _output_get (Variables|Default|SetActive Active))
  (if _output_get
    (Rendering|SetActorHiddenInGame false)
    (Collision|SetCollisionEnabled _checkpointcollider "QueryOnly")
    (else
      (Rendering|SetActorHiddenInGame true)
      (Collision|SetCollisionEnabled _checkpointcollider "NoCollision"))))

(event EventBeginPlay
  (CallFunction|ToggleCheckpoint (Variables|Default|GetActive)))

(event Collision|EventActorBeginOverlap
  (params (OtherActor :type Actor%20Object%20Reference)))

(event EventTick
  (params (DeltaSeconds :type Float%20%28single-precision%29)))

(fn ConstructionScript)