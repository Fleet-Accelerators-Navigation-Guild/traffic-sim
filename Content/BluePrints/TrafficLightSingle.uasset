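; Single traffic light actor that cycles itself from BeginPlay by showing one of its red, yellow or green light components at a time.
; A looping FlipFlop and Delay chain starts on yellow, then repeats green, yellow, red, skipping yellow between red and green.
; Each switch function also sets the boolean TrafficLightState, true only on green.
; The construction script sets default phase durations, and setter functions can change them.
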(event EventBeginPlay
  (CallFunction|SwitchtoYellow :!label _label)
  (Utilities|FlowControl|Delay (Math|Conversions|ToFloat(Integer) (Variables|Default|GetyellowTiming)))
  (Utilities|FlowControl|FlipFlop :!label _label_2
    (:A
      (CallFunction|SwitchtoGreen)
      (Utilities|FlowControl|Delay (Math|Conversions|ToFloat(Integer) (Variables|Default|GetgreenTiming)))
      (goto _label))
    (:B
      (CallFunction|SwitchtoRed)
      (Utilities|FlowControl|Delay (Math|Conversions|ToFloat(Integer) (Variables|Default|GetredTiming)))
      (goto _label_2))))

(event Collision|EventActorBeginOverlap
  (params (OtherActor :type Actor%20Object%20Reference)))

(event EventTick
  (params (DeltaSeconds :type Float%20%28single-precision%29)))

(fn ConstructionScript
  (Variables|Default|SetredTiming 10)
  (Variables|Default|SetyellowTiming 2)
  (Variables|Default|SetgreenTiming 10))

(fn SwitchtoYellow
  (Variables|Default|SettrafficLightState false)
  (Utilities|FlowControl|Sequence
    (:then_0
      (Development|SetHiddeninGame (Variables|Default|GetyellowLight) false false))
    (:then_1
      (Development|SetHiddeninGame (Variables|Default|GetredLight) true false))))

(fn SwitchtoGreen
  (Variables|Default|SettrafficLightState true)
  (Utilities|FlowControl|Sequence
    (:then_0
      (Development|SetHiddeninGame (Variables|Default|GetgreenLight) false false))
    (:then_1
      (Development|SetHiddeninGame (Variables|Default|GetredLight) true false))))

(fn SwitchtoRed
  (Variables|Default|SettrafficLightState false)
  (Utilities|FlowControl|Sequence
    (:then_0
      (Development|SetHiddeninGame (Variables|Default|GetredLight) false false))
    (:then_1
      (Development|SetHiddeninGame (Variables|Default|GetgreenLight) true false))))

(fn SetYellowTiming
  (params (time :type Integer))
  (Variables|Default|SetyellowTiming time))

(fn SetRedTiming
  (params (time :type Integer))
  (Variables|Default|SetredTiming time))

(fn SetGreenTiming
  (params (time :type Integer))
  (Variables|Default|SetgreenTiming time))