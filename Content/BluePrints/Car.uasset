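; Unfinished car Blueprint, apparently intended to drive itself along roads and detect nearby actors.
; Construction enables gravity on CarBox; Drive issues SimpleMoveToLocation toward TempDestination, while MakeConeOfSight stores box-overlap results in DetectedActors.
; GetRoad's nearest-actor destination assignment is disconnected, Brake and CheckTurn are empty stubs, and the event graph calls none of these functions.
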(event EventBeginPlay)

(event Collision|EventActorBeginOverlap
  (params (OtherActor :type Actor%20Object%20Reference)))

(event EventTick
  (params (DeltaSeconds :type Float%20%28single-precision%29)))

(fn ConstructionScript
  (Physics|SetEnableGravity (Variables|Default|GetCarBox) true))

(fn Drive
  (AI|Navigation|SimpleMovetoLocation 0 (Variables|Default|Gettemp%20destination)))

(fn MakeConeOfSight
  (bind _returnvalue (Transformation|GetActorLocation))
  (bind (_outactors _returnvalue_2) (Collision|BoxOverlapActors _returnvalue (+ (Math|Rotator|GetRotationXVector (Math|Conversions|RotationFromXVector _returnvalue)) (Variables|Default|GetBox%20Extent)) (Variables|Default|GetObject%20Types) (Variables|Default|GetActor%20Class%20Filter) (Utilities|Array|MakeArray (Components|GetOwner) 0) :!class /Script/Engine.KismetSystemLibrary))
  (Variables|Default|SetdetectedActors _outactors)
  (LocalVariables|SetNewLocalVar_0 _returnvalue_2))

(fn Brake)

(fn GetRoad
  (bind _outactors (Actor|GetAllActorsOfClass 0)))

(fn CheckTurn)