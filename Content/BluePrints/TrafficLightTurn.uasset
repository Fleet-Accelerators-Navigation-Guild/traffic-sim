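; Traffic light actor with a main signal and a turn-arrow signal, alternating between their phases.
; From BeginPlay, a looping FlipFlop runs a green, yellow, red cycle for the main lights, then one for the arrows, using Delays.
; Switch functions toggle light component visibility and set a state boolean for each signal, true only on green.
; Construction script sets default timings and hides the yellow and green arrows; setters can change each timing.
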(event EventBeginPlay
  (Utilities|FlowControl|FlipFlop :!label _label
    (:A
      (CallFunction|SwitchtoGreen)
      (Utilities|FlowControl|Delay (Math|Conversions|ToFloat(Integer) (Variables|Default|GetgreenTiming)))
      (CallFunction|SwitchtoYellow)
      (Utilities|FlowControl|Delay (Math|Conversions|ToFloat(Integer) (Variables|Default|GetyellowTiming)))
      (CallFunction|SwitchtoRed)
      (Utilities|FlowControl|Delay (Math|Conversions|ToFloat(Integer) (Variables|Default|GetredTiming)))
      (goto _label))
    (:B
      (CallFunction|SwitchtoGreenArrow)
      (Utilities|FlowControl|Delay (Math|Conversions|ToFloat(Integer) (Variables|Default|GetgreenArrowTiming)))
      (CallFunction|SwitchtoYellowArrow)
      (Utilities|FlowControl|Delay (Math|Conversions|ToFloat(Integer) (Variables|Default|GetyellowArrowTiming)))
      (CallFunction|SwitchtoRedArrow)
      (Utilities|FlowControl|Delay (Math|Conversions|ToFloat(Integer) (Variables|Default|GetredArrowTiming)))
      (goto _label))))

(event Collision|EventActorBeginOverlap
  (params (OtherActor :type Actor%20Object%20Reference)))

(event EventTick
  (params (DeltaSeconds :type Float%20%28single-precision%29)))

(fn ConstructionScript
  (Variables|Default|SetredTiming 10)
  (Variables|Default|SetyellowTiming 2)
  (Variables|Default|SetgreenTiming 10)
  (Variables|Default|SetredArrowTiming 7)
  (Variables|Default|SetyellowArrowTiming 2)
  (Variables|Default|SetgreenArrowTiming 7)
  (Development|SetHiddeninGame (Variables|Default|GetyellowArrow) true false))

(fn SetRedTiming
  (params (time :type Integer))
  (Variables|Default|SetredTiming time))

(fn SetYellowTiming
  (params (time :type Integer))
  (Variables|Default|SetyellowTiming time))

(fn SetGreenTiming
  (params (time :type Integer))
  (Variables|Default|SetgreenTiming time))

(fn SwitchtoRed
  (Variables|Default|SettrafficLightState false)
  (Utilities|FlowControl|Sequence
    (:then_0
      (Development|SetHiddeninGame (Variables|Default|GetredLight) false false))
    (:then_1
      (Development|SetHiddeninGame (Variables|Default|GetgreenLight) true false))))

(fn SwitchtoGreen
  (Variables|Default|SettrafficLightState true)
  (Utilities|FlowControl|Sequence
    (:then_0
      (Development|SetHiddeninGame (Variables|Default|GetgreenLight) false false))
    (:then_1
      (Development|SetHiddeninGame (Variables|Default|GetredLight) true false))))

(fn SwitchtoYellow
  (Variables|Default|SettrafficLightState false)
  (Utilities|FlowControl|Sequence
    (:then_0
      (Development|SetHiddeninGame (Variables|Default|GetyellowLight) false false))
    (:then_1
      (Development|SetHiddeninGame (Variables|Default|GetredLight) true false))))

(fn SetRedArrowTiming
  (params (time :type Integer))
  (Variables|Default|SetredArrowTiming time))

(fn SetYellowArrowTiming
  (params (time :type Integer))
  (Variables|Default|SetyellowArrowTiming time))

(fn SetGreenArrowTiming
  (params (time :type Integer))
  (Variables|Default|SetgreenArrowTiming time))

(fn SwitchtoRedArrow
  (Variables|Default|SettrafficLightStateArrow false)
  (Utilities|FlowControl|Sequence
    (:then_0
      (Development|SetHiddeninGame (Variables|Default|GetredArrow) false false))
    (:then_1
      (Development|SetHiddeninGame (Variables|Default|GetyellowArrow) true false))))

(fn SwitchtoGreenArrow
  (Variables|Default|SettrafficLightStateArrow true)
  (Utilities|FlowControl|Sequence
    (:then_0
      (Development|SetHiddeninGame (Variables|Default|GetgreenArrow) false false))
    (:then_1
      (Development|SetHiddeninGame (Variables|Default|GetredArrow) true false))))

(fn SwitchtoYellowArrow
  (Variables|Default|SettrafficLightStateArrow false)
  (Utilities|FlowControl|Sequence
    (:then_0
      (Development|SetHiddeninGame (Variables|Default|GetyellowArrow) false false))
    (:then_1
      (Development|SetHiddeninGame (Variables|Default|GetredArrow) true false))))